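; Player controller that manages the local player's main HUD and reacts to game-state timer and quit events.
; On BeginPlay it creates HUD_Main if a locally controlled pawn is already possessed, then binds to two BP_GameStateMain events.
; The end-game-time event feeds minutes and seconds to the HUD timer widget, and the quit event exits the game.
; Unpossessing collapses the HUD.
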(event Custom|CreateWidget
  (bind _returnvalue (Pawn|GetControlledPawn))
  (Utilities|IsValid _returnvalue
    (:Is%20Valid
      (if (Pawn|IsLocallyControlled _returnvalue)
        (bind _returnvalue_2 (UserInterface|CreateWidget "/Game/NURZ/UI/HUD_Main.HUD_Main_C" self))
        (bind _output_get (Variables|Default|SetHUD%20Ref _returnvalue_2))
        (UserInterface|Viewport|AddtoViewport _output_get 0)))))

(event Custom|EndGameTime
  (params (M :type Float%20%28double-precision%29) (S :type Float%20%28double-precision%29))
  (bind _hud_ref (Variables|Default|GetHUD%20Ref)
    (:then
      (Default|SetTimer (Variables|/Game/NURZ/UI/HUD_Main.HUD_Main_C|GetW_Timer _hud_ref) M S))
    (:else)))

(event Custom|TimerEnd
  (CallFunction|QuitGame))

(event Custom|QuitGame
  (Game|QuitGame self "Quit" false))

(event EventBeginPlay
  (CallFunction|CreateWidget)
  (bind _asbp_game_state_main (Utilities|Casting|CastToBP_GameStateMain (Game|GetGameState)))
  (EventDispatchers|BindEventtoEndGameTime _asbp_game_state_main (delegate Custom|EndGameTime))
  (EventDispatchers|BindEventtoQuitGame _asbp_game_state_main (delegate Custom|TimerEnd)))

(event EventUnPossess
  (params (UnpossessedPawn :type Pawn%20Object%20Reference))
  (bind _hud_ref (Variables|Default|GetHUD%20Ref)
    (:then
      (Widget|SetVisibility _hud_ref "Collapsed"))
    (:else)))

(fn ConstructionScript)