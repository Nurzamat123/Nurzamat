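; GA_AutoFire is a gameplay ability intended for automatic fire, but its ActivateAbility event is empty.
; The FIRE event asks the avatar's ability system component to activate abilities by tag, allowing remote activation.
; A disconnected, never-executed chain would run FIRE on a looping server-authority timer, then clear it and end the ability on input release.
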(event Custom|FIRE
  (Abilities|TryActivateAbilitiesbyTag (Ability|GetAbilitySystemComponent (.AvatarActor (Utilities|Struct|BreakGameplayAbilityActorInfo (Ability|GetActorInfo)))) (Variables|Default|GetGameplay%20Tag%20Container) true))

(event Ability|EventActivateAbility)