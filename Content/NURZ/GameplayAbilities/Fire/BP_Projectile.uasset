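; Projectile actor in the Fire gameplay abilities folder that delivers a GAS damage effect on overlap.
; On BeginPlay it sets its life span to the movement component's initial speed divided by Range.
; Overlaps ignore the instigator; on authority, characters with a valid ability system component receive the damage effect spec and the projectile is destroyed.
; It also destroys itself on non-character hits and on any non-instigator overlap on remotes.
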(event OnComponentBeginOverlap(Collision)
  (params (OverlappedComponent :type Primitive%20Component%20Object%20Reference) (OtherActor :type Actor%20Object%20Reference) (OtherComp :type Primitive%20Component%20Object%20Reference) (OtherBodyIndex :type Integer) (bFromSweep :type Boolean) (SweepResult :type Hit%20Result%20Structure%20%28by%20ref%29))
  (if (!= OtherActor (Game|GetInstigator))
    (Networking|SwitchHasAuthority
      (:Authority
        (bind _asbp_third_person_character (Utilities|Casting|CastToBP_ThirdPersonCharacter OtherActor)
          (:then
            (if (Utilities|IsValid (Ability|GetAbilitySystemComponent _asbp_third_person_character))
              (GameplayEffects|ApplyGameplayEffectSpecToSelf (Ability|GetAbilitySystemComponent _asbp_third_person_character) (Variables|Default|GetDamageEffectSpecHandle))
              (Actor|DestroyActor)))
          (:CastFailed
            (Actor|DestroyActor :!label _label))))
      (:Remote
        (goto _label)))))

(event EventBeginPlay
  ;[1 1 1] Set life span
  (Actor|SetLifeSpan (/ (Variables|/Script/Engine.ProjectileMovementComponent|GetInitialSpeed (Variables|Default|GetProjectileMovement)) (Variables|Default|GetRange))))

(fn ConstructionScript)