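; Gameplay ability that cycles the third-person character to its next weapon.
; On authority only, it advances the weapon component's current index with wraparound, then calls a Multicast event that runs EquipWeapon.
; The index passed to that event is recomputed after the increment, so it points one past the stored index.
; The ability ends after a short placeholder delay for animation, and CommitAbility is left unwired.
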(event Custom|Multicast
  (params (WeaponIndex :type Integer) (Target :type Weapon%20Component%20Object%20Reference))
  (Class|WeaponComponent|EquipWeapon Target WeaponIndex))

(event Ability|EventActivateAbility
  (Ability|HasAuthority
    (:True
      (Development|PrintString "Hello")
      (bind _asbp_third_person_character (Utilities|Casting|CastToBP_ThirdPersonCharacter (Ability|GetAvatarActorfromActorInfo)))
      (Variables|Default|SetWeapon%20Component (Variables|/Script/Nurzamat.NURZCharacter|GetWeaponComponent _asbp_third_person_character))
      (Variables|/Script/Nurzamat.WeaponComponent|SetCurrentWeaponIndex (Variables|/Script/Nurzamat.NURZCharacter|GetWeaponComponent _asbp_third_person_character) (Math|Integer|%(Integer) (+ (Variables|/Script/Nurzamat.WeaponComponent|GetCurrentWeaponIndex (Variables|/Script/Nurzamat.NURZCharacter|GetWeaponComponent _asbp_third_person_character)) 1) (Utilities|Array|Length (Variables|/Script/Nurzamat.WeaponComponent|GetWeapons (Variables|/Script/Nurzamat.NURZCharacter|GetWeaponComponent _asbp_third_person_character)))))
      (CallFunction|Multicast (Math|Integer|%(Integer) (+ (Variables|/Script/Nurzamat.WeaponComponent|GetCurrentWeaponIndex (Variables|/Script/Nurzamat.NURZCharacter|GetWeaponComponent _asbp_third_person_character)) 1) (Utilities|Array|Length (Variables|/Script/Nurzamat.WeaponComponent|GetWeapons (Variables|/Script/Nurzamat.NURZCharacter|GetWeaponComponent _asbp_third_person_character)))) (Variables|/Script/Nurzamat.NURZCharacter|GetWeaponComponent _asbp_third_person_character))
      ;[1 0 0.02387] animation must be
      (Utilities|FlowControl|Delay 0.2)
      (Ability|EndAbility))))