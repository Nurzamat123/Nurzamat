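; Gameplay ability that lets the third-person character sprint while its input is held.
; On activation it ends at once if the character has the ADS tag; otherwise it caches the current walk speed and adds a sprint bonus to it.
; A wait-for-input-release task ends the ability, and ending restores the cached speed to the movement component.
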(event Ability|EventActivateAbility
  (bind _asbp_third_person_character (Utilities|Casting|CastToBP_ThirdPersonCharacter (Ability|GetAvatarActorfromActorInfo)))
  (bind _output_get (Variables|Default|SetOwningActor _asbp_third_person_character))
  (if (GameplayTags|HasTag (Variables|/Game/ThirdPerson/Blueprints/BP_ThirdPersonCharacter.BP_ThirdPersonCharacter_C|GetGameplay%20Tag%20Container _output_get) "(TagName=\"Ability.ADS\")" true)
    (Ability|EndAbility)
    (else
      (Variables|Default|SetMax%20Walk%20Speed%20Default (Variables|/Script/Engine.CharacterMovementComponent|GetMaxWalkSpeed (Variables|/Script/Engine.Character|GetCharacterMovement _output_get)))
      (Variables|/Script/Engine.CharacterMovementComponent|SetMaxWalkSpeed (Variables|/Script/Engine.Character|GetCharacterMovement _output_get) (+ (Variables|Default|GetMax%20Walk%20Speed%20Default) (Variables|Default|GetAddSprintSpeed)))
      (Ability|Tasks|WaitInputRelease true
        (:OnRelease
          (Ability|EndAbility))))))

(event Ability|EventOnEndAbility
  (params (bWasCancelled :type Boolean))
  (Variables|/Script/Engine.CharacterMovementComponent|SetMaxWalkSpeed (Variables|/Script/Engine.Character|GetCharacterMovement (Variables|Default|GetOwningActor)) (Variables|Default|GetMax%20Walk%20Speed%20Default)))